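; Floor spike trap that raises its spikes when a BP_Pickup actor enters its Box collision.
; Tick moves the Spikes component up by SpikeSpeed per frame, then back down, between height limits set in the construction script.
; At the top it reverses and calls HitBySpikeTrap on the single pickup found at BeginPlay, without rechecking overlap.
; Movement is not scaled by delta time.
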(event `self.ReceiveBeginPlay`
  ;[0 0.8359 1] Gets ref to pickup
  (bind _returnvalue (`GameplayStatics.GetActorOfClass` "/Game/VehicleVarietyPack/Blueprints/Pickup/BP_Pickup.BP_Pickup_C"))
  (set `self.pickupRef` _returnvalue))

(event `self.ReceiveTick`
  (params (DeltaSeconds :type "Float (single-precision)"))
  (bind _spikes (`self.Spikes`))
  (bind _x (.x (`SceneComponent.K2_GetComponentLocation` _spikes)))
  (bind _y (.y (`SceneComponent.K2_GetComponentLocation` _spikes)))
  (bind _z (.z (`SceneComponent.K2_GetComponentLocation` _spikes)))
  ;[1 0.6328 0] Moves 'Spikes' component up/down when needed
  (if (<= (`self.zPosMax`) _z)
    (set `self.IsSpikeMovingUp` false)
    (`/Game/VehicleVarietyPack/Blueprints/Pickup/BP_Pickup.HitBySpikeTrap` (`self.pickupRef`)))
  (if (`self.IsSpikeMovingUp`)
    (`SceneComponent.K2_SetWorldLocation` _spikes (`KismetMathLibrary.MakeVector` _x _y (+ _z (`self.SpikeSpeed`))) false false)
    (elif (< (`self.zPosMin`) _z)
      (`SceneComponent.K2_SetWorldLocation` _spikes (`KismetMathLibrary.MakeVector` _x _y (- _z (`self.SpikeSpeed`))) false false))))

(event `self.Box.OnComponentBeginOverlap`
  (params (OverlappedComponent :type "PrimitiveComponent Object Reference") (OtherActor :type "Actor Object Reference") (OtherComp :type "PrimitiveComponent Object Reference") (OtherBodyIndex :type Integer) (bFromSweep :type Boolean) (SweepResult :type "HitResult Structure (by ref)"))
  ;[0 0.6953 1] Pickup collides with collison box on spike trap
  (if (`self.IsSpikeMovingUp`)
    _
    (elif (`KismetMathLibrary.ClassIsChildOf` (`GameplayStatics.GetObjectClass` OtherActor) "/Game/VehicleVarietyPack/Blueprints/Pickup/BP_Pickup.BP_Pickup_C")
      (set `self.IsSpikeMovingUp` true))))

(fn `UserConstructionScript`
  (bind _z (.z (`SceneComponent.K2_GetComponentLocation` (`self.Spikes`))))
  (set `self.zPosMin` _z)
  (set `self.zPosMax` (+ _z 30.0)))