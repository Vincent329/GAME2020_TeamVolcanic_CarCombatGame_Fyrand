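; BP_Bullet is a projectile actor that damages turrets.
; When its Hitbox overlaps a BP_Turret, it plays a hit sound at the world origin, subtracts DamageValue from the turret's CurrentHealth and destroys itself.
; Tick runs a short Delay, then destroys the bullet if SMBullet is valid, acting as a lifetime limit.
; The Velocity-based movement code is disconnected, so this graph does not move the bullet.
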(event `self.ReceiveTick`
  (params (DeltaSeconds :type "Float (single-precision)"))
  ;[1 0.3047 0] movement
  (`KismetSystemLibrary.Delay` 3.0)
  (`/Engine/EditorBlueprintResources/StandardMacros.IsValid` (`self.SM_Bullet`)
    (:`Is Valid`
      (`self.K2_DestroyActor`)
      (`KismetSystemLibrary.PrintString` "dead bullet"))))

(event `self.Hitbox.OnComponentBeginOverlap`
  (params (OverlappedComponent :type "PrimitiveComponent Object Reference") (OtherActor :type "Actor Object Reference") (OtherComp :type "PrimitiveComponent Object Reference") (OtherBodyIndex :type Integer) (bFromSweep :type Boolean) (SweepResult :type "HitResult Structure (by ref)"))
  (bind _asbp_turret (cast `/Game/Fyrand/Turret/BP_Turret` OtherActor))
  (`GameplayStatics.PlaySoundAtLocation` "/Game/Fyrand/Turret/Hitturret.Hitturret" (0.0 0.0 0.0) (struct) 1.0 1.0 0.0 null null null)
  (bind _output_get (set `/Game/Fyrand/Turret/BP_Turret.Current Health` (- (`/Game/Fyrand/Turret/BP_Turret.Current Health` _asbp_turret) (`self.Damage Value`)) _asbp_turret))
  (`KismetSystemLibrary.PrintString` (`KismetStringLibrary.Conv_DoubleToString` _output_get))
  (`self.K2_DestroyActor`))

(fn `UserConstructionScript`)