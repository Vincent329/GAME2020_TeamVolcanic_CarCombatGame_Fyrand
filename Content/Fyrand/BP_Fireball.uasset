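; Fireball projectile actor that climbs, then dives toward a stored target position and explodes on the ground.
; Spawn stores the target and flips the pitch; Tick moves it manually by Velocity and Acceleration.
; Above a Z threshold, Tick re-aims velocity at the target, zeroes acceleration and rotates the fireball to match.
; Box overlap with named landscape actors (lava only while descending) spawns BP_Fireball_Explosion once, then destroys the fireball after a delay.
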(event `self.ReceiveTick`
  (params (DeltaSeconds :type "Float (single-precision)"))
  (bind _returnvalue (`SceneComponent.K2_GetComponentLocation` (`self.DefaultSceneRoot`)))
  ;[1 0 0.3047] Movement
  (set `self.Velocity` (+ (`self.Acceleration`) (`self.Velocity`)))
  (`SceneComponent.K2_SetWorldLocation` (`self.DefaultSceneRoot`) (+ (`SceneComponent.K2_GetComponentLocation` (`self.DefaultSceneRoot`)) (`self.Velocity`)) false false)
  ;[1 0 0.7734] Change velocity to aim towards player once the fireball hits a high enough Z value
  (if (> (.z _returnvalue) 6800.0)
    (bind _output_get (set `self.Velocity` (* (* (- (`self.PickupPos`) _returnvalue) (`GameplayStatics.GetWorldDeltaSeconds`)) 0.5)))
    (set `self.Acceleration` (0.0 0.0 0.0))
    (`SceneComponent.K2_SetRelativeRotation` (`self.DefaultSceneRoot`) (`KismetMathLibrary.MakeRotFromX` (`KismetMathLibrary.MakeVector` (.x _output_get) (.y _output_get) (* (.z _output_get) -1.0))) false false)))

(event `self.Box.OnComponentBeginOverlap`
  (params (OverlappedComponent :type "PrimitiveComponent Object Reference") (OtherActor :type "Actor Object Reference") (OtherComp :type "PrimitiveComponent Object Reference") (OtherBodyIndex :type Integer) (bFromSweep :type Boolean) (SweepResult :type "HitResult Structure (by ref)"))
  (bind _returnvalue (`KismetSystemLibrary.GetDisplayName` OtherActor))
  ;[1 0.5156 0] Collision with ground -> spawn explosion
  (if (and (or (and (< (.z (`self.Velocity`)) 0.0) (`KismetStringLibrary.EqualEqual_StrStr` _returnvalue "LavaLandscapeHazard")) (`KismetStringLibrary.EqualEqual_StrStr` _returnvalue "GroundLandscape")) (not (`self.Exploding`)))
    (set `self.Exploding` true)
    (`|SpawnActorFromClass` "/Game/Fyrand/BP_Fireball_Explosion.BP_Fireball_Explosion_C" (`KismetMathLibrary.MakeTransform` (`KismetMathLibrary.MakeVector` (.x (.location (`self.GetTransform`))) (.y (.location (`self.GetTransform`))) (+ (.z (.location (`self.GetTransform`))) 150.0)) (.rotation (`self.GetTransform`)) (.scale (`self.GetTransform`))) "Undefined" "OverrideRootScale" null null)
    (`KismetSystemLibrary.Delay` 1.0)
    (`self.K2_DestroyActor`)))

(fn `Spawn`
  (params (pos :type "Vector Structure"))
  (set `self.PickupPos` pos)
  (`SceneComponent.K2_SetRelativeRotation` (`self.DefaultSceneRoot`) (`KismetMathLibrary.MakeRotator` 0.0 180.0) false false))

(fn `UserConstructionScript`)