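; BP_Geyser is a geyser actor that periodically spawns BP_Fireball actors.
; On BeginPlay it caches a reference to a BP_Pickup found in the level.
; A frame counter on Tick, so tied to frame rate, spawns a fireball at the geyser's root whenever it reaches its maximum, then resets.
; Each fireball's Spawn function receives the pickup mesh's current world location.
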(event `self.ReceiveBeginPlay`
  (bind _returnvalue (`GameplayStatics.GetActorOfClass` "/Game/VehicleVarietyPack/Blueprints/Pickup/BP_Pickup.BP_Pickup_C"))
  (set `self.PickupRef` _returnvalue))

(event `self.ReceiveTick`
  (params (DeltaSeconds :type "Float (single-precision)"))
  (bind _fireballtimer (`self.FireballTimer`))
  ;[1 0.5859 0] Fireball spawning
  (set `self.FireballTimer` (+ _fireballtimer 1))
  (if (>= _fireballtimer (`self.FireballTimerMax`))
    (bind _returnvalue (`|SpawnActorFromClass` "/Game/Fyrand/BP_Fireball.BP_Fireball_C" (`KismetMathLibrary.MakeTransform` (`SceneComponent.K2_GetComponentLocation` (`self.DefaultSceneRoot`))) "Undefined" "OverrideRootScale" null null))
    (`/Game/Fyrand/BP_Fireball.Spawn` _returnvalue (`SceneComponent.K2_GetComponentLocation` (`WheeledVehicle.Mesh` (`self.PickupRef`))))
    (set `self.FireballTimer` 0)))

(fn `UserConstructionScript`)