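; BP_Turret is an enemy turret that detects BP_Pickup pawns through PawnSensing, turns to face them and shoots.
; Sightings rotate it immediately, while a delay paces bullet spawning from BulletSpawner with gunfire sound and later destroys the bullet.
; ModifyHealth applies clamped damage.
; Tick updates the EnemyHealth widget bar and calls CheckHealth, which plays a destruction sound once at zero health, then removes the turret.
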(event `self.ReceiveBeginPlay`)

(event `self.PawnSensing.OnSeePawn`
  (params (Pawn :type "Pawn Object Reference"))
  (bind _asbp_pickup (cast `/Game/VehicleVarietyPack/Blueprints/Pickup/BP_Pickup` Pawn))
  (`|ExecutionSequence`
    (:`then_0`
      (`self.K2_SetActorRotation` (`ActorComponent.GetOwner` (`self.Turret`)) (`KismetMathLibrary.FindLookAtRotation` (`self.K2_GetActorLocation`) (`self.K2_GetActorLocation` _asbp_pickup)) false))
    (:`then_1`
      (`KismetSystemLibrary.Delay` 1.0)
      (bind _returnvalue (`|SpawnActorFromClass` "/Game/Fyrand/Turret/BP_TurretBullet.BP_TurretBullet_C" (`SceneComponent.K2_GetComponentToWorld` (`self.BulletSpawner`)) "Undefined" "OverrideRootScale" null null))
      (`GameplayStatics.PlaySound2D` "/Game/VehicleVarietyPack/Blueprints/Pickup/SoundCues/Gunfire_Sound.Gunfire_Sound" 1.0 1.0 0.0 null null)
      (`KismetSystemLibrary.Delay` 2.0)
      (`/Engine/EditorBlueprintResources/StandardMacros.IsValid` _returnvalue
        (:`Is Valid`
          (`self.K2_DestroyActor` _returnvalue))))))

(event `self.ReceiveTick`
  (params (DeltaSeconds :type "Float (single-precision)"))
  (`self.Check Health`)
  (bind _asenemy_health (cast `/Game/MenuAssets/EnemyHealth` (`WidgetComponent.GetUserWidgetObject` (`self.Widget`))))
  (`ProgressBar.SetPercent` (`/Game/MenuAssets/EnemyHealth.ProgressBar_65` _asenemy_health) (/ (`self.TurretHealth`) (`self.FullHealth`))))

(event `Check Health`
  (if (<= (`self.TurretHealth`) 0.0)
    (`/Engine/EditorBlueprintResources/StandardMacros.DoOnce` false
      (:`Completed`
        (`GameplayStatics.PlaySoundAtLocation` "/Game/Fyrand_Sound/TurretDestroyed.TurretDestroyed" (0.0 0.0 0.0) (struct) 1.0 1.0 0.0 null null null)
        (`KismetSystemLibrary.Delay` 0.5)
        (`self.K2_DestroyActor`)))))

(fn `Modify Health`
  (params (HealthToSubtract :type "Float (double-precision)"))
  (set `self.TurretHealth` (`KismetMathLibrary.FClamp` (- (`self.TurretHealth`) HealthToSubtract) 0.0 (`self.FullHealth`))))

(fn `UserConstructionScript`)