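; Player-driven pickup truck pawn with a camera-aimed gun, horn, flip reset, HUD and pause menu.
; Spike traps, fireballs and timer-throttled lava overlaps reduce health; CheckHealth triggers Death, which disables input, then shows a game-over menu.
; Tick scales engine pitch with RPM and, when a CharSplinePath start reports collision, teleports the truck along that spline until near its last point.
; CharSplinePath actors are gathered in the Construction Script.
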(event `self.ReceiveBeginPlay`
  ;[0.8047 1 0] UI
  (bind _returnvalue (`|CreateWidget` "/Game/MenuAssets/UserInterface.UserInterface_C"))
  (`UserWidget.AddToViewport` _returnvalue 0))

(event `InputAxis|Forward`
  (params (AxisValue :type "Float (single-precision)"))
  ;[0.1216 0.9263 1] vehicle movement
  (`WheeledVehicleMovementComponent.SetThrottleInput` (`self.VehicleMovement`) AxisValue))

(event `InputAxis|Turn`
  (params (AxisValue :type "Float (single-precision)"))
  ;[0.1216 0.9263 1] vehicle movement
  (`WheeledVehicleMovementComponent.SetSteeringInput` (`self.VehicleMovement`) AxisValue))

(event `Key|LeftShift`
  (params (Key :type "Key Structure"))
  (bind _vehiclemovement (`self.VehicleMovement`))
  ;[0.1216 0.9263 1] vehicle movement
  (:`Pressed`
    (`WheeledVehicleMovementComponent.SetHandbrakeInput` _vehiclemovement true))
  (:`Released`
    (`WheeledVehicleMovementComponent.SetHandbrakeInput` _vehiclemovement false)))

(event `self.ReceiveTick`
  (params (DeltaSeconds :type "Float (single-precision)"))
  (bind _lavadamagetimer (`self.LavaDamageTimer`))
  (bind _splineref (`self.SplineRef`))
  (bind _returnvalue (* (`self.SplineVelocity`) (`self.SplineConstSpeed`)))
  (bind _returnvalue_2 (`SceneComponent.K2_GetComponentLocation` (`self.Mesh`)))
  ;[0 0.5078 1] Lava Hazard
  (if (> _lavadamagetimer 0)
    (set `self.LavaDamageTimer` (- _lavadamagetimer 1))
    (elif (`self.CollidingWithLava`)
      (`self.CollidesWithLava`)
      (set `self.LavaDamageTimer` (`self.LavaDamageTimerMax`))))
  ;[0.8984 0 1] Engine Roar
  (`AudioComponent.SetPitchMultiplier` (`self.Engine`) (`KismetMathLibrary.FClamp` (/ (`WheeledVehicleMovementComponent.GetEngineRotationSpeed` (`self.VehicleMovement`)) 4000.0) 0.0 1000.0))
  ;[0.003793 0.04688 0.007606] Splines
  (if (`self.MovingOnSpline`)
    ;;[0.1016 0 1] Teleport the vehicle along the spline
    (`self.K2_TeleportTo` (`SplineComponent.FindLocationClosestToWorldLocation` (`self.SplineRef`) (+ _returnvalue _returnvalue_2) "World") (`KismetMathLibrary.MakeRotator` 0.0 0.0 (`self.StartYaw`)))
    (if (and (< (`KismetMathLibrary.Abs` (.y (- (`SplineComponent.GetLocationAtSplinePoint` _splineref (- (`SplineComponent.GetNumberOfSplinePoints` _splineref) 1) "World") _returnvalue_2))) (`KismetMathLibrary.Abs` (.y (* _returnvalue 20)))) (< (`KismetMathLibrary.Abs` (.x (- (`SplineComponent.GetLocationAtSplinePoint` _splineref (- (`SplineComponent.GetNumberOfSplinePoints` _splineref) 1) "World") _returnvalue_2))) (`KismetMathLibrary.Abs` (.x (* _returnvalue 20)))))
      ;;[0 0.01562 1] Exit Spline
      (set `self.MovingOnSpline` false)
      (set `self.splineCounter` 0)
      (set `self.SplineRef` null)
      (set `self.SplineVelocity` (0.0 0.0 0.0)))
    (else
      ;;[1 0.3281 0] check for collision with a spline start
      (for _array_element (`self.CharSplineArray`)
        (if (`/Game/Fyrand/CharSplinePath.Collision` _array_element)
          ;;[0 1 0.8359] Start of spline movement
          (set `self.StartYaw` (.yaw (`SceneComponent.K2_GetComponentRotation` (`self.Mesh`))))
          (set `self.SplineRef` (`/Game/Fyrand/CharSplinePath.Spline` _array_element))
          (set `self.MovingOnSpline` true)
          (set `self.SplineVelocity` (* (- (`SplineComponent.GetLocationAtSplinePoint` (`self.SplineRef`) 0 "World") (`SceneComponent.K2_GetComponentLocation` (`self.Mesh`))) (`GameplayStatics.GetWorldDeltaSeconds`))))))))

(event `InputAction|Pause`
  (params (Key :type "Key Structure"))
  ;[0.125 0 1] Pause the Game
  (:`Pressed`
    (`self.PauseGame`)))

(event `InputAxis|MouseY`
  (params (AxisValue :type "Float (single-precision)"))
  ;[1 0 0.1641] vehicle camera control and gun aiming
  (`self.AddControllerPitchInput` (* AxisValue -1.0)))

(event `InputAction|Honk`
  (params (Key :type "Key Structure"))
  (bind _honking (`self.Honking`))
  ;[0 1 0.4375] Honk the Horn
  (:`Pressed`
    (`AudioComponent.Play` _honking 0.0))
  (:`Released`
    (`AudioComponent.Stop` _honking)))

(event `InputAxis|MouseX`
  (params (AxisValue :type "Float (single-precision)"))
  ;[1 0 0.1641] vehicle camera control and gun aiming
  (`self.AddControllerYawInput` AxisValue)
  (`SceneComponent.K2_SetWorldRotation` (`self.SM_KA47_X`) (`SceneComponent.GetSocketRotation` (`self.Camera`) "None") false false))

(event `InputAction|Reset Vehicle`
  (params (Key :type "Key Structure"))
  (bind _mesh (`self.Mesh`))
  ;[0.3828 1 0] Spacebar -> Flip Vehicle
  (:`Pressed`
    (`self.K2_TeleportTo` (`KismetMathLibrary.MakeVector` (.x (`SceneComponent.K2_GetComponentLocation` _mesh)) (.y (`SceneComponent.K2_GetComponentLocation` _mesh)) (+ (.z (`SceneComponent.K2_GetComponentLocation` _mesh)) 80.0)) (`KismetMathLibrary.MakeRotator` 0.0 0.0 (.yaw (`SceneComponent.K2_GetComponentRotation` _mesh))))))

(event `InputAction|Fire`
  (params (Key :type "Key Structure"))
  (bind _aimpointer (`self.AimPointer`))
  ;[0 0.1328 1] Fire bullets
  (:`Pressed`
    (`|SpawnActorFromClass` "/Game/Fyrand/BP_Bullet.BP_Bullet_C" (`KismetMathLibrary.MakeTransform` (`SceneComponent.K2_GetComponentLocation` _aimpointer) (`SceneComponent.K2_GetComponentRotation` _aimpointer) (0.1 0.1 0.1)) "Undefined" "OverrideRootScale" null null)
    (`GameplayStatics.PlaySoundAtLocation` "/Game/VehicleVarietyPack/Blueprints/Pickup/SoundCues/Gunfire_Sound.Gunfire_Sound" (0.0 0.0 0.0) (struct) 1.0 1.0 0.0 null null null)))

(event `Check Health`
  ;[0.5938 0 1] Checking Health Event
  (if (<= (`self.CurrentHealth`) 0.0)
    (`self.Death`)
    (`KismetSystemLibrary.Delay` 1.0)
    (`self.Game Over Menu`)))

(event `self.CollisionBox.OnComponentBeginOverlap`
  (params (OverlappedComponent :type "PrimitiveComponent Object Reference") (OtherActor :type "Actor Object Reference") (OtherComp :type "PrimitiveComponent Object Reference") (OtherBodyIndex :type Integer) (bFromSweep :type Boolean) (SweepResult :type "HitResult Structure (by ref)"))
  ;[1 0.2344 0] Collsion - Lava / Fireball
  (if (`KismetStringLibrary.EqualEqual_StrStr` (`KismetSystemLibrary.GetDisplayName` OtherActor) "LavaLandscapeHazard")
    (set `self.CollidingWithLava` true)
    (`KismetSystemLibrary.PrintString` "Lava col start"))
  (if (`KismetMathLibrary.ClassIsChildOf` (`GameplayStatics.GetObjectClass` OtherActor) "/Game/Fyrand/BP_Fireball.BP_Fireball_C")
    (`self.HitByFireball`)))

(event `self.CollisionBox.OnComponentEndOverlap`
  (params (OverlappedComponent :type "PrimitiveComponent Object Reference") (OtherActor :type "Actor Object Reference") (OtherComp :type "PrimitiveComponent Object Reference") (OtherBodyIndex :type Integer))
  ;[1 0.2344 0] Collsion - Lava / Fireball
  (if (`KismetStringLibrary.EqualEqual_StrStr` (`KismetSystemLibrary.GetDisplayName` OtherActor) "LavaLandscapeHazard")
    (set `self.CollidingWithLava` false)
    (`KismetSystemLibrary.PrintString` "Lava col end")))

(fn `CollidesWithLava`
  (`KismetSystemLibrary.PrintString` "LAVA HOT")
  (set `self.CurrentHealth` (- (`self.CurrentHealth`) 5.0))
  (`self.Check Health`))

(fn `Death`
  (`MovementComponent.StopMovementImmediately` (`self.VehicleMovement`))
  (`self.DisableInput` (`GameplayStatics.GetPlayerController` 0)))

(fn `Game Over Menu`
  (`GameplayStatics.SetGamePaused` true)
  (`/Engine/EditorBlueprintResources/StandardMacros.IsValid` (`self.GameOverMenu`)
    (:`Is Valid`
      _)
    (:`Is Not Valid`
      (bind _returnvalue (`|CreateWidget` "/Game/MenuAssets/GameOver.GameOver_C" (`GameplayStatics.GetPlayerController` 0)))
      (set `self.GameOverMenu` _returnvalue)))
  (`UserWidget.AddToViewport` (`self.GameOverMenu`) 0)
  (`WidgetBlueprintLibrary.SetInputMode_UIOnlyEx` (`GameplayStatics.GetPlayerController` 0) (`self.GameOverMenu`))
  (set `PlayerController.bShowMouseCursor` true (`GameplayStatics.GetPlayerController` 0)))

(fn `HitByFireball`
  (`KismetSystemLibrary.PrintString` "Fireball hot")
  (set `self.CurrentHealth` (- (`self.CurrentHealth`) 20.0))
  (`self.Check Health`))

(fn `HitBySpikeTrap`
  (bind _vehiclemovement (`self.VehicleMovement`))
  (`KismetSystemLibrary.PrintString` "Pickup takes damage or something")
  (set `MovementComponent.Velocity` (/ (`MovementComponent.Velocity` _vehiclemovement) (2.0 2.0 2.0)) _vehiclemovement)
  (set `self.CurrentHealth` (- (`self.CurrentHealth`) 5.0))
  (`self.Check Health`))

(fn `PauseGame`
  (`GameplayStatics.SetGamePaused` true)
  (`/Engine/EditorBlueprintResources/StandardMacros.IsValid` (`self.PauseMenu`)
    (:`Is Valid`
      _)
    (:`Is Not Valid`
      (bind _returnvalue (`|CreateWidget` "/Game/MenuAssets/PauseMenu.PauseMenu_C" (`GameplayStatics.GetPlayerController` 0)))
      (set `self.PauseMenu` _returnvalue)))
  (`UserWidget.AddToViewport` (`self.PauseMenu`) 0)
  (`WidgetBlueprintLibrary.SetInputMode_UIOnlyEx` (`GameplayStatics.GetPlayerController` 0) (`self.PauseMenu`))
  (set `PlayerController.bShowMouseCursor` true (`GameplayStatics.GetPlayerController` 0)))

(fn `UnpauseGame`
  (bind _returnvalue (`GameplayStatics.GetPlayerController` 0))
  (`GameplayStatics.SetGamePaused` false)
  (`WidgetLayoutLibrary.RemoveAllWidgets`)
  (`WidgetBlueprintLibrary.SetInputMode_GameOnly` _returnvalue)
  (set `PlayerController.bShowMouseCursor` false _returnvalue)
  (bind _returnvalue_2 (`|CreateWidget` "/Game/MenuAssets/UserInterface.UserInterface_C"))
  (`UserWidget.AddToViewport` _returnvalue_2 0))

(fn `UserConstructionScript`
  (bind _outactors (`GameplayStatics.GetAllActorsOfClass` "/Game/Fyrand/CharSplinePath.CharSplinePath_C"))
  (set `self.CharSplineArray` _outactors)
  (set `self.CurrentHealth` (`self.FullHealth`)))