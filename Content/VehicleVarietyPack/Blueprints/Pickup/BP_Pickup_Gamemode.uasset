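; Game mode for the pickup vehicle that runs a minutes-and-seconds countdown and ends the game when time runs out.
; Tick feeds a one-second latent Delay, so the timer steps about once per second and rolls seconds over into minutes.
; When both reach zero, it calls Death on the player's BP_Pickup pawn, waits briefly, clears all widgets and calls that pawn's GameOverMenu.
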(event `self.ReceiveTick`
  (params (DeltaSeconds :type "Float (single-precision)"))
  (`KismetSystemLibrary.Delay` 1.0)
  (set `self.TimeSec` (- (`self.TimeSec`) 1))
  (if (< (`self.TimeSec`) 0)
    (set `self.TimeMin` (- (`self.TimeMin`) 1))
    (set `self.TimeSec` 59))
  ;[0.3125 1 0] If Time is Up
  (if (== (`self.TimeSec`) 0)
    (if (== (`self.TimeMin`) 0)
      ;[0.9219 0 1] Generates Game Over Screen
      (bind _asbp_pickup (cast `/Game/VehicleVarietyPack/Blueprints/Pickup/BP_Pickup` (`GameplayStatics.GetPlayerPawn` 0)))
      (`/Game/VehicleVarietyPack/Blueprints/Pickup/BP_Pickup.Death` _asbp_pickup)
      (`KismetSystemLibrary.Delay` 1.5)
      (`WidgetLayoutLibrary.RemoveAllWidgets`)
      (`/Game/VehicleVarietyPack/Blueprints/Pickup/BP_Pickup.Game Over Menu` _asbp_pickup))))

(fn `UserConstructionScript`)