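; BP_geyser_hazard is a moving effect actor that behaves like a projectile, spawning a tinted shockwave particle on BeginPlay.
; Tick moves it along local X by Speed scaled by a timeline curve, and counts Duration down.
; A Delay loop started by timeline updates disables box collision when Duration expires, then destroys the actor.
; Overlapping an actor whose first tag isn't "ky_shot" spawns HitFx and destroys it immediately.
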(event `self.ReceiveBeginPlay`
  (bind _defaultsceneroot (`self.DefaultSceneRoot`))
  ;[0.1484 0 1] spawn shot shockwave
  (bind _returnvalue (`GameplayStatics.SpawnEmitterAtLocation` "/Game/FXVarietyPack/Particles/P_ky_shotShockwave.P_ky_shotShockwave" (`SceneComponent.K2_GetComponentLocation` _defaultsceneroot) (`SceneComponent.K2_GetComponentRotation` _defaultsceneroot)))
  (`ParticleSystemComponent.SetVectorParameter` _returnvalue "color" (`KismetMathLibrary.Conv_LinearColorToVector` (`self.color`)))
  ;[0.007812 1 0] effect move correct
  (bind (_direction _valuecorrect) (`Timeline|Timeline_0`)
    (:`Update`
      (set `self.speedCorrect` _valuecorrect)
      ;[1 0 0.1875] duration control
      (`KismetSystemLibrary.Delay` 0.1 :!label _label)
      (if (< (`self.duration`) 0.0)
        ;[0.9219 1 0] fx deactivate
        (`PrimitiveComponent.SetCollisionEnabled` (`self.Box`) "NoCollision")
        (`KismetSystemLibrary.Delay` 1.0)
        ;[0.6406 1 0] effect destroy
        (`self.K2_DestroyActor`)
        (else
          (goto _label))))))

(event `self.ReceiveTick`
  (params (DeltaSeconds :type "Float (single-precision)"))
  ;[0 1 0.3906] duration increment for control
  (set `self.duration` (- (`self.duration`) DeltaSeconds))
  ;[1 0 0.3047] move control
  (`self.K2_AddActorLocalOffset` (`KismetMathLibrary.MakeVector` (* (`self.speed`) (`self.speedCorrect`) (`GameplayStatics.GetWorldDeltaSeconds`)))))

(event `self.ReceiveActorBeginOverlap`
  (params (OtherActor :type "Actor Object Reference"))
  ;[1 0.9375 0] spawn collison fx
  (if (`KismetSystemLibrary.IsValid` OtherActor)
    (if (!= (`|GetArrayItem` (`Actor.Tags` OtherActor)) "ky_shot")
      (`GameplayStatics.SpawnEmitterAtLocation` (`self.hitFx`) (`SceneComponent.K2_GetComponentLocation` (`self.Box`)))
      ;[0.1016 1 0] fx destroy
      (`self.K2_DestroyActor`))))

(fn `UserConstructionScript`)